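; BP_BlackHole is an actor that exposes the look of a black hole effect as Blueprint variables.
; Its Construction Script copies each variable into a named scalar or vector parameter on the BlackHole component's materials, covering size, event horizon, rings, disk colour, Doppler, emission and quality steps.
; The graph contains no other logic, so the visual effect itself comes from those materials.
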(fn ConstructionScript
  (Rendering|Material|SetScalarParameterValueonMaterials (Variables|Default|GetBlackHole) "BlackHoleSize" (Variables|HoleParameters|GetBlack%20Hole%20Size))
  (Rendering|Material|SetScalarParameterValueonMaterials (Variables|Default|GetBlackHole) "maxrot(create duplicates)" (Variables|Misc|Getmaxrot%28create%20duplicates%29))
  (Rendering|Material|SetScalarParameterValueonMaterials (Variables|Default|GetBlackHole) "Ring_Intensity" (Variables|RingParameters|GetRing_Intensity))
  (Rendering|Material|SetScalarParameterValueonMaterials (Variables|Default|GetBlackHole) "Ring_Radius" (Variables|RingParameters|GetRing_Radius))
  (Rendering|Material|SetScalarParameterValueonMaterials (Variables|Default|GetBlackHole) "Ring_Speed" (Variables|RingParameters|GetRing_Speed))
  (Rendering|Material|SetScalarParameterValueonMaterials (Variables|Default|GetBlackHole) "rrad" (Variables|Misc|Getrrad))
  (Rendering|Material|SetScalarParameterValueonMaterials (Variables|Default|GetBlackHole) "Texture_Stretch" (Variables|Misc|GetTexture_Stretch))
  (Rendering|Material|SetScalarParameterValueonMaterials (Variables|Default|GetBlackHole) "Doppler_Intensity" (Variables|RingParameters|GetDoppler_Intensity))
  (Rendering|Material|SetScalarParameterValueonMaterials (Variables|Default|GetBlackHole) "Emission Intensity" (Variables|HoleParameters|GetEmission%20Intensity))
  (Rendering|Material|SetScalarParameterValueonMaterials (Variables|Default|GetBlackHole) "iring" (Variables|RingParameters|GetRing_Emission))
  (Rendering|Material|SetScalarParameterValueonMaterials (Variables|Default|GetBlackHole) "rfac" (Variables|Misc|Getrfac))
  (Rendering|Material|SetScalarParameterValueonMaterials (Variables|Default|GetBlackHole) "Ring_Intensity_Falloff" (Variables|RingParameters|GetRing_Intensity_Falloff))
  (Rendering|Material|SetScalarParameterValueonMaterials (Variables|Default|GetBlackHole) "rint" (Variables|RingParameters|GetRings_Amount))
  (Rendering|Material|SetScalarParameterValueonMaterials (Variables|Default|GetBlackHole) "Quality_Steps" (Variables|Misc|GetQuality_Steps))
  (Rendering|Material|SetScalarParameterValueonMaterials (Variables|Default|GetBlackHole) "Event_Horizon_Size" (Variables|HoleParameters|GetEvent_Horizon_Size))
  (Rendering|Material|SetScalarParameterValueonMaterials (Variables|Default|GetBlackHole) "rv" (Variables|Misc|Getrv))
  (Rendering|Material|SetVectorParameterValueonMaterials (Variables|Default|GetBlackHole) "Disk Colour" (Variables|HoleParameters|GetDisk%20Colour)))