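; BP_Galaxy is a placeable actor that renders a configurable galaxy particle effect through a Niagara component.
; Its Construction Script assigns the chosen Niagara system, resetting override parameters, then pushes the actor's variables into matching user parameters.
; These cover spawning, sprite size, torus shape, drag, vortex and curl-noise motion, and two colours.
; The event graph holds only disabled placeholder events, so the Blueprint adds no runtime logic.
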(event EventBeginPlay)

(event Collision|EventActorBeginOverlap
  (params (OtherActor :type Actor%20Object%20Reference)))

(event EventTick
  (params (DeltaSeconds :type Float%20%28single-precision%29)))

(fn ConstructionScript
  (Class|NiagaraComponent|SetAsset (Variables|Default|GetNiagara) (Variables|Default|GetNiagaraSystem) true)
  (Effects|Components|ParticleSystem|SetFloatParameter (Variables|Default|GetNiagara) "SpawnRate" (Variables|Default|GetSpawnRate))
  (Effects|Components|ParticleSystem|SetFloatParameter (Variables|Default|GetNiagara) "Lifetime" (Variables|Default|GetLifetime))
  (Effects|Components|ParticleSystem|SetFloatParameter (Variables|Default|GetNiagara) "SpriteSizeMin" (Variables|Default|GetSpriteSizeMin))
  (Effects|Components|ParticleSystem|SetFloatParameter (Variables|Default|GetNiagara) "SpriteSizeMax" (Variables|Default|GetSpriteSizeMax))
  (Effects|Components|ParticleSystem|SetFloatParameter (Variables|Default|GetNiagara) "TorusLargeRadius" (Variables|Default|GetTorusLargeRadius))
  (Effects|Components|ParticleSystem|SetFloatParameter (Variables|Default|GetNiagara) "TorusHandleRadius" (Variables|Default|GetTorusHandleRadius))
  (Effects|Components|ParticleSystem|SetFloatParameter (Variables|Default|GetNiagara) "Drag" (Variables|Default|GetDrag))
  (Effects|Components|ParticleSystem|SetFloatParameter (Variables|Default|GetNiagara) "VortexForce" (Variables|Default|GetVortexForce))
  (Effects|Components|ParticleSystem|SetFloatParameter (Variables|Default|GetNiagara) "CurlNoise" (Variables|Default|GetCurlNoise))
  (Effects|Components|ParticleSystem|SetVectorParameter (Variables|Default|GetNiagara) "VortexAxis" (Variables|Default|GetVortexAxis))
  (Effects|Components|ParticleSystem|SetColorParameter (Variables|Default|GetNiagara) "Colour1" (Variables|Default|GetColour1))
  (Effects|Components|ParticleSystem|SetColorParameter (Variables|Default|GetNiagara) "Colour2" (Variables|Default|GetColour2)))