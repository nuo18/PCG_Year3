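; BP_Skybox is a skybox actor that displays a configurable texture on a sphere mesh using the MSkyBox material.
; Its construction script assigns the material to the sphere and creates a dynamic instance from it.
; It then pushes the actor's brightness, HDRI Cons, rotation axis and angle, tint and texture variables into that instance.
; The event graph holds only disabled stub events, so all setup happens at construction.
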(event EventBeginPlay)

(event Collision|EventActorBeginOverlap
  (params (OtherActor :type Actor%20Object%20Reference)))

(event EventTick
  (params (DeltaSeconds :type Float%20%28single-precision%29)))

(fn ConstructionScript
  (Rendering|Material|SetMaterial (Variables|Default|GetSphere) 0 (Variables|Default|GetM_SkyBox))
  (bind _returnvalue (Rendering|Material|CreateDynamicMaterialInstance (Variables|Default|GetSphere) 0 (Variables|Default|GetM_SkyBox) "None" :!class /Script/Engine.PrimitiveComponent))
  (Variables|Default|SetDyn_M_Skybox _returnvalue)
  (Rendering|Material|SetScalarParameterValue (Variables|Default|GetDyn_M_Skybox) "HDRI Brightness" (Variables|Default|GetHDRI%20Brightness) :!class /Script/Engine.MaterialInstanceDynamic)
  (Rendering|Material|SetScalarParameterValue (Variables|Default|GetDyn_M_Skybox) "HDRI Cons" (Variables|Default|GetHDRI%20Cons) :!class /Script/Engine.MaterialInstanceDynamic)
  (Rendering|Material|SetScalarParameterValue (Variables|Default|GetDyn_M_Skybox) "RotationAngle" (Variables|Default|GetRotationAngle) :!class /Script/Engine.MaterialInstanceDynamic)
  (Rendering|Material|SetVectorParameterValue (Variables|Default|GetDyn_M_Skybox) "RotationAxis" (Math|Conversions|ToLinearColor(Vector) (Variables|Default|GetRotation%20Axis)) :!class /Script/Engine.MaterialInstanceDynamic)
  (Rendering|Material|SetVectorParameterValue (Variables|Default|GetDyn_M_Skybox) "Tint" (Variables|Default|GetTint) :!class /Script/Engine.MaterialInstanceDynamic)
  (Rendering|Material|SetTextureParameterValue (Variables|Default|GetDyn_M_Skybox) "Texture" (Variables|Default|GetTexture)))