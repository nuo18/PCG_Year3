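; Parent planet actor that builds a configurable planet look from body, cloud, atmosphere and ring components, with no active runtime logic.
; The construction script creates a dynamic material on the body, feeding variables into noise, liquid and primary and secondary surface layer parameters.
; It then assigns cloud, atmosphere and ring materials and sets their parameters per component.
; Body and clouds share NoiseScale, and the ring's Sparsity targets a parameter named None.
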(event EventBeginPlay)

(event Collision|EventActorBeginOverlap
  (params (OtherActor :type Actor%20Object%20Reference)))

(event EventTick
  (params (DeltaSeconds :type Float%20%28single-precision%29)))

(fn ConstructionScript
  ;[0.15 0.15 0.15 0.5] Planet Body
  (bind _returnvalue (Rendering|Material|CreateDynamicMaterialInstance (Variables|Default|GetPlanet_Body) 0 (Variables|Materials|GetM_Planet_Body) "None" :!class /Script/Engine.PrimitiveComponent))
  (Variables|DynamicMaterials|SetDyn_M_Planet_Body _returnvalue)
  (Rendering|Material|SetScalarParameterValue (Variables|DynamicMaterials|GetDyn_M_Planet_Body) "Noise Bias" (Variables|BodyBlending|GetNoise%20Bias) :!class /Script/Engine.MaterialInstanceDynamic)
  (Rendering|Material|SetScalarParameterValue (Variables|DynamicMaterials|GetDyn_M_Planet_Body) "Noise Contrast" (Variables|BodyBlending|GetNoise%20Contrast) :!class /Script/Engine.MaterialInstanceDynamic)
  (Rendering|Material|SetScalarParameterValue (Variables|DynamicMaterials|GetDyn_M_Planet_Body) "NoiseOffset X" (Variables|BodyBlending|GetNoiseOffset%20X) :!class /Script/Engine.MaterialInstanceDynamic)
  (Rendering|Material|SetScalarParameterValue (Variables|DynamicMaterials|GetDyn_M_Planet_Body) "NoiseOffset Y" (Variables|BodyBlending|GetNoiseOffset%20Y) :!class /Script/Engine.MaterialInstanceDynamic)
  (Rendering|Material|SetScalarParameterValue (Variables|DynamicMaterials|GetDyn_M_Planet_Body) "NoiseOffset Z" (Variables|BodyBlending|GetNoiseOffset%20Z) :!class /Script/Engine.MaterialInstanceDynamic)
  (Rendering|Material|SetScalarParameterValue (Variables|DynamicMaterials|GetDyn_M_Planet_Body) "NoiseScale" (Variables|BodyBlending|GetNoiseScale) :!class /Script/Engine.MaterialInstanceDynamic)
  (Rendering|Material|SetScalarParameterValue (Variables|DynamicMaterials|GetDyn_M_Planet_Body) "Liquid Noise Bias" (Variables|BodyLiquid|GetLiquid%20Noise%20Bias) :!class /Script/Engine.MaterialInstanceDynamic)
  (Rendering|Material|SetScalarParameterValue (Variables|DynamicMaterials|GetDyn_M_Planet_Body) "Liquid Noise Contrast" (Variables|BodyLiquid|GetLiquid%20Noise%20Contrast) :!class /Script/Engine.MaterialInstanceDynamic)
  (Rendering|Material|SetScalarParameterValue (Variables|DynamicMaterials|GetDyn_M_Planet_Body) "Liquid Noise Scale" (Variables|BodyLiquid|GetLiquid%20Noise%20Scale) :!class /Script/Engine.MaterialInstanceDynamic)
  (Rendering|Material|SetTextureParameterValue (Variables|DynamicMaterials|GetDyn_M_Planet_Body) "Liquid Normal" (Variables|BodyLiquid|GetLiquid%20Normal))
  (Rendering|Material|SetScalarParameterValue (Variables|DynamicMaterials|GetDyn_M_Planet_Body) "Liquid Ripple Intensity" (Variables|BodyLiquid|GetLiquid%20Ripple%20Intensity) :!class /Script/Engine.MaterialInstanceDynamic)
  (Rendering|Material|SetScalarParameterValue (Variables|DynamicMaterials|GetDyn_M_Planet_Body) "Liquid Ripple Scale" (Variables|BodyLiquid|GetLiquid%20Ripple%20Scale) :!class /Script/Engine.MaterialInstanceDynamic)
  (Rendering|Material|SetScalarParameterValue (Variables|DynamicMaterials|GetDyn_M_Planet_Body) "Liquid Speed X" (Variables|BodyLiquid|GetLiquid%20Speed%20X) :!class /Script/Engine.MaterialInstanceDynamic)
  (Rendering|Material|SetScalarParameterValue (Variables|DynamicMaterials|GetDyn_M_Planet_Body) "Liquid Speed Y" (Variables|BodyLiquid|GetLiquid%20Speed%20Y) :!class /Script/Engine.MaterialInstanceDynamic)
  (Rendering|Material|SetScalarParameterValue (Variables|DynamicMaterials|GetDyn_M_Planet_Body) "Liquid Brightness" (Variables|BodyLiquid|GetLiquid%20Brightness) :!class /Script/Engine.MaterialInstanceDynamic)
  (Rendering|Material|SetVectorParameterValue (Variables|DynamicMaterials|GetDyn_M_Planet_Body) "Liquid Colour" (Variables|BodyLiquid|GetLiquid%20Colour) :!class /Script/Engine.MaterialInstanceDynamic)
  (Rendering|Material|SetScalarParameterValue (Variables|DynamicMaterials|GetDyn_M_Planet_Body) "Liquid Metallic" (Variables|BodyLiquid|GetLiquid%20Metallic) :!class /Script/Engine.MaterialInstanceDynamic)
  (Rendering|Material|SetScalarParameterValue (Variables|DynamicMaterials|GetDyn_M_Planet_Body) "Liquid Roughness" (Variables|BodyLiquid|GetLiquid%20Roughness) :!class /Script/Engine.MaterialInstanceDynamic)
  (Rendering|Material|SetTextureParameterValue (Variables|DynamicMaterials|GetDyn_M_Planet_Body) "Primary Albedo" (Variables|BodyPrimary|GetPrimary%20Albedo))
  (Rendering|Material|SetVectorParameterValue (Variables|DynamicMaterials|GetDyn_M_Planet_Body) "Primary Colour" (Variables|BodyPrimary|GetPrimary%20Colour) :!class /Script/Engine.MaterialInstanceDynamic)
  (Rendering|Material|SetScalarParameterValue (Variables|DynamicMaterials|GetDyn_M_Planet_Body) "Primary Desaturation" (Variables|BodyPrimary|GetPrimary%20Desaturation) :!class /Script/Engine.MaterialInstanceDynamic)
  (Rendering|Material|SetTextureParameterValue (Variables|DynamicMaterials|GetDyn_M_Planet_Body) "Primary Height" (Variables|BodyPrimary|GetPrimary%20Height))
  (Rendering|Material|SetScalarParameterValue (Variables|DynamicMaterials|GetDyn_M_Planet_Body) "Primary Metallic" (Variables|BodyPrimary|GetPrimary%20Metallic) :!class /Script/Engine.MaterialInstanceDynamic)
  (Rendering|Material|SetTextureParameterValue (Variables|DynamicMaterials|GetDyn_M_Planet_Body) "Primary Normal" (Variables|BodyPrimary|GetPrimary%20Normal))
  (Rendering|Material|SetTextureParameterValue (Variables|DynamicMaterials|GetDyn_M_Planet_Body) "Primary ORM" (Variables|BodyPrimary|GetPrimary%20ORM))
  (Rendering|Material|SetScalarParameterValue (Variables|DynamicMaterials|GetDyn_M_Planet_Body) "Primary Roughness" (Variables|BodyPrimary|GetPrimary%20Roughness) :!class /Script/Engine.MaterialInstanceDynamic)
  (Rendering|Material|SetScalarParameterValue (Variables|DynamicMaterials|GetDyn_M_Planet_Body) "Primary Scale" (Variables|BodyPrimary|GetPrimary%20Scale) :!class /Script/Engine.MaterialInstanceDynamic)
  (Rendering|Material|SetTextureParameterValue (Variables|DynamicMaterials|GetDyn_M_Planet_Body) "Secondary Albedo" (Variables|BodySecondary|GetSecondary%20Albedo))
  (Rendering|Material|SetVectorParameterValue (Variables|DynamicMaterials|GetDyn_M_Planet_Body) "Secondary Colour" (Variables|BodySecondary|GetSecondary%20Colour) :!class /Script/Engine.MaterialInstanceDynamic)
  (Rendering|Material|SetScalarParameterValue (Variables|DynamicMaterials|GetDyn_M_Planet_Body) "Secondary Desaturation" (Variables|BodySecondary|GetSecondary%20Desaturation) :!class /Script/Engine.MaterialInstanceDynamic)
  (Rendering|Material|SetScalarParameterValue (Variables|DynamicMaterials|GetDyn_M_Planet_Body) "Secondary Metallic" (Variables|BodySecondary|GetSecondary%20Metallic) :!class /Script/Engine.MaterialInstanceDynamic)
  (Rendering|Material|SetTextureParameterValue (Variables|DynamicMaterials|GetDyn_M_Planet_Body) "Secondary Normal" (Variables|BodySecondary|GetSecondary%20Normal))
  (Rendering|Material|SetTextureParameterValue (Variables|DynamicMaterials|GetDyn_M_Planet_Body) "Secondary ORM" (Variables|BodySecondary|GetSecondary%20ORM))
  (Rendering|Material|SetScalarParameterValue (Variables|DynamicMaterials|GetDyn_M_Planet_Body) "Secondary Roughness" (Variables|BodySecondary|GetSecondary%20Roughness) :!class /Script/Engine.MaterialInstanceDynamic)
  (Rendering|Material|SetScalarParameterValue (Variables|DynamicMaterials|GetDyn_M_Planet_Body) "Secondary Scale" (Variables|BodySecondary|GetSecondary%20Scale) :!class /Script/Engine.MaterialInstanceDynamic)
  ;[0.15 0.15 0.15 0.5] Materials
  (Rendering|Material|SetMaterial (Variables|Default|GetPlanet_Clouds) 0 (Variables|Materials|GetM_Planet_Clouds))
  (Rendering|Material|SetMaterial (Variables|Default|GetPlanet_Atmosphere) 0 (Variables|Materials|GetM_Planet_Atmosphere))
  (Rendering|Material|SetMaterial (Variables|Default|GetPlanet_Ring) 0 (Variables|Materials|GetM_Planet_Ring))
  ;[0.15 0.15 0.15 0.5] Rings
  (Rendering|Material|SetScalarParameterValueonMaterials (Variables|Default|GetPlanet_Ring) "Freq" (Variables|Rings|GetFrequency))
  (Rendering|Material|SetScalarParameterValueonMaterials (Variables|Default|GetPlanet_Ring) "Glow" (Variables|Rings|GetGlow))
  (Rendering|Material|SetScalarParameterValueonMaterials (Variables|Default|GetPlanet_Ring) "InnerRingDensity" (Variables|Rings|GetInnerRingDensity))
  (Rendering|Material|SetScalarParameterValueonMaterials (Variables|Default|GetPlanet_Ring) "InnerRingExtent" (Variables|Rings|GetInnerRingExtent))
  (Rendering|Material|SetScalarParameterValueonMaterials (Variables|Default|GetPlanet_Ring) "Intensity" (Variables|Rings|GetIntensity))
  (Rendering|Material|SetScalarParameterValueonMaterials (Variables|Default|GetPlanet_Ring) "Master Opacity" (Variables|Rings|GetMaster%20Opacity))
  (Rendering|Material|SetScalarParameterValueonMaterials (Variables|Default|GetPlanet_Ring) "Offset" (Variables|Rings|GetOffset))
  (Rendering|Material|SetScalarParameterValueonMaterials (Variables|Default|GetPlanet_Ring) "OuterRingDensity" (Variables|Rings|GetOuterRingDensity))
  (Rendering|Material|SetScalarParameterValueonMaterials (Variables|Default|GetPlanet_Ring) "OuterRingExtent" (Variables|Rings|GetOuterRingExtent))
  (Rendering|Material|SetScalarParameterValueonMaterials (Variables|Default|GetPlanet_Ring) "None" (Variables|Rings|GetSparsity))
  (Rendering|Material|SetVectorParameterValueonMaterials (Variables|Default|GetPlanet_Ring) "Colour1" (Variables|Rings|GetRing_Colour1))
  (Rendering|Material|SetVectorParameterValueonMaterials (Variables|Default|GetPlanet_Ring) "Colour2" (Variables|Rings|GetRing_Colour2))
  ;[0.15 0.15 0.15 0.5] Clouds
  (Rendering|Material|SetScalarParameterValueonMaterials (Variables|Default|GetPlanet_Clouds) "Cloud Cutoff" (Variables|Clouds|GetCloud%20Cutoff))
  (Rendering|Material|SetScalarParameterValueonMaterials (Variables|Default|GetPlanet_Clouds) "Colour Blend Multiplier" (Variables|Clouds|GetColour%20Blend%20Multiplier))
  (Rendering|Material|SetScalarParameterValueonMaterials (Variables|Default|GetPlanet_Clouds) "Distortion Amount" (Variables|Clouds|GetDistortion%20Amount))
  (Rendering|Material|SetScalarParameterValueonMaterials (Variables|Default|GetPlanet_Clouds) "Distortion Scale" (Variables|Clouds|GetDistortion%20Scale))
  (Rendering|Material|SetScalarParameterValueonMaterials (Variables|Default|GetPlanet_Clouds) "Edge Definition" (Variables|Clouds|GetEdge%20Definition))
  (Rendering|Material|SetScalarParameterValueonMaterials (Variables|Default|GetPlanet_Clouds) "Master Opactiy" (Variables|Clouds|GetMaster%20Opactiy))
  (Rendering|Material|SetScalarParameterValueonMaterials (Variables|Default|GetPlanet_Clouds) "Noise Scale" (Variables|Clouds|GetNoise%20Scale))
  (Rendering|Material|SetVectorParameterValueonMaterials (Variables|Default|GetPlanet_Clouds) "ColourEdge" (Variables|Clouds|GetColourEdge))
  (Rendering|Material|SetVectorParameterValueonMaterials (Variables|Default|GetPlanet_Clouds) "UV Divisors x,y,z" (Variables|Clouds|GetUV%20Divisors%20x,y,z))
  (Rendering|Material|SetVectorParameterValueonMaterials (Variables|Default|GetPlanet_Clouds) "ColourMain" (Variables|Clouds|GetColourMain))
  (Rendering|Material|SetVectorParameterValueonMaterials (Variables|Default|GetPlanet_Clouds) "Speed" (Variables|Clouds|GetSpeed))
  ;[0.15 0.15 0.15 0.5] Atmosphere
  (Rendering|Material|SetScalarParameterValueonMaterials (Variables|Default|GetPlanet_Atmosphere) "Colour Blend Multiplier" (Variables|Atmosphere|GetAtmos_Blend))
  (Rendering|Material|SetScalarParameterValueonMaterials (Variables|Default|GetPlanet_Atmosphere) "Inner Extent" (Variables|Atmosphere|GetInner%20Extent))
  (Rendering|Material|SetScalarParameterValueonMaterials (Variables|Default|GetPlanet_Atmosphere) "Inner Falloff" (Variables|Atmosphere|GetInner%20Falloff))
  (Rendering|Material|SetScalarParameterValueonMaterials (Variables|Default|GetPlanet_Atmosphere) "Master Opacity" (Variables|Atmosphere|GetAtmos%20Master%20Opacity))
  (Rendering|Material|SetScalarParameterValueonMaterials (Variables|Default|GetPlanet_Atmosphere) "Outer Extent" (Variables|Atmosphere|GetOuter%20Extent))
  (Rendering|Material|SetScalarParameterValueonMaterials (Variables|Default|GetPlanet_Atmosphere) "Outer Falloff" (Variables|Atmosphere|GetOuter%20Falloff))
  (Rendering|Material|SetVectorParameterValueonMaterials (Variables|Default|GetPlanet_Atmosphere) "Colour1" (Variables|Atmosphere|GetAtmos%20Colour1))
  (Rendering|Material|SetVectorParameterValueonMaterials (Variables|Default|GetPlanet_Atmosphere) "Colour2" (Variables|Atmosphere|GetAtmos%20Colour2)))