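; Asteroid belt region actor that procedurally scatters asteroids within a box volume using PCG.
; The construction script sizes the box from PCGRegion and pushes seed, count, scale, offset and density settings into the PCG graph instance.
; It then calls ForceRegen to force a local PCG regeneration; the event graph is unused.
; The ScaleMax setter shows no parameter name, unlike the other setters.
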(event EventBeginPlay)

(event Collision|EventActorBeginOverlap
  (params (OtherActor :type Actor%20Object%20Reference)))

(event EventTick
  (params (DeltaSeconds :type Float%20%28single-precision%29)))

(fn ConstructionScript
  (Components|Box|SetBoxExtent (Variables|Default|GetBox) (Variables|Default|GetPCG_Region) true)
  (Utilities|FlowControl|Sequence
    (:then_0
      (Effects|Components|ParticleSystem|SetFloatParameter (Variables|/Script/PCG.PCGComponent|GetGraphInstance (Variables|Default|GetPCG)) "ScaleMin" (Variables|Default|GetScale%20Min))
      (Effects|Components|ParticleSystem|SetFloatParameter (Variables|/Script/PCG.PCGComponent|GetGraphInstance (Variables|Default|GetPCG)) "ScaleMax" (Variables|Default|GetScale%20Max))
      (Class|PCGGraphParametersHelpers|SetInt32Parameter (Variables|/Script/PCG.PCGComponent|GetGraphInstance (Variables|Default|GetPCG)) "Seed" (Variables|Default|GetSeed))
      (Class|PCGGraphParametersHelpers|SetInt32Parameter (Variables|/Script/PCG.PCGComponent|GetGraphInstance (Variables|Default|GetPCG)) "NumOfAsteroids" (Variables|Default|GetNum%20Of%20Asteroids))
      (Effects|Components|ParticleSystem|SetFloatParameter (Variables|/Script/PCG.PCGComponent|GetGraphInstance (Variables|Default|GetPCG)) "OffsetMinX" (Variables|Default|GetOffset%20Min%20X))
      (Effects|Components|ParticleSystem|SetFloatParameter (Variables|/Script/PCG.PCGComponent|GetGraphInstance (Variables|Default|GetPCG)) "OffsetMinY" (Variables|Default|GetOffset%20Min%20Y))
      (Effects|Components|ParticleSystem|SetFloatParameter (Variables|/Script/PCG.PCGComponent|GetGraphInstance (Variables|Default|GetPCG)) "OffsetMinZ" (Variables|Default|GetOffset%20Min%20Z))
      (Effects|Components|ParticleSystem|SetFloatParameter (Variables|/Script/PCG.PCGComponent|GetGraphInstance (Variables|Default|GetPCG)) "OffsetMaxX" (Variables|Default|GetOffset%20Max%20X))
      (Effects|Components|ParticleSystem|SetFloatParameter (Variables|/Script/PCG.PCGComponent|GetGraphInstance (Variables|Default|GetPCG)) "OffsetMaxY" (Variables|Default|GetOffset%20Max%20Y))
      (Effects|Components|ParticleSystem|SetFloatParameter (Variables|/Script/PCG.PCGComponent|GetGraphInstance (Variables|Default|GetPCG)) "OffsetMaxZ" (Variables|Default|GetOffset%20Max%20Z))
      (Effects|Components|ParticleSystem|SetFloatParameter (Variables|/Script/PCG.PCGComponent|GetGraphInstance (Variables|Default|GetPCG)) "Density" (Variables|Default|GetDensity)))
    (:then_1
      (CallFunction|ForceRegen))))

(fn ForceRegen
  (Class|PCGComponent|GenerateLocal (Variables|Default|GetPCG) true)
  (return))