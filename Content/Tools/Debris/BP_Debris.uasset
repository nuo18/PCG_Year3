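; BP_Debris is a tool actor that generates debris procedurally with a PCG component inside an adjustable box.
; The construction script sizes the box from BoxExtents and pushes the voxel size, density, offset range, scale range and seed into the PCG graph instance's parameters.
; It then calls ForceRegen, which forces a local PCG generation, so the result rebuilds whenever construction reruns.
; The event graph has no active logic.
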(event EventBeginPlay)

(event Collision|EventActorBeginOverlap
  (params (OtherActor :type Actor%20Object%20Reference)))

(event EventTick
  (params (DeltaSeconds :type Float%20%28single-precision%29)))

(fn ConstructionScript
  (Components|Box|SetBoxExtent (Variables|Default|GetBox) (Variables|Default|GetBox%20Extents) true)
  (Utilities|FlowControl|Sequence
    (:then_0
      (Effects|Components|ParticleSystem|SetFloatParameter (Variables|/Script/PCG.PCGComponent|GetGraphInstance (Variables|Default|GetPCG)) "Voxelsize" (Variables|Default|GetVoxelSize))
      (Effects|Components|ParticleSystem|SetFloatParameter (Variables|/Script/PCG.PCGComponent|GetGraphInstance (Variables|Default|GetPCG)) "Density" (Variables|Default|GetDensity))
      (Effects|Components|ParticleSystem|SetFloatParameter (Variables|/Script/PCG.PCGComponent|GetGraphInstance (Variables|Default|GetPCG)) "OffsetMin" (Variables|Default|GetOffset%20Min))
      (Effects|Components|ParticleSystem|SetFloatParameter (Variables|/Script/PCG.PCGComponent|GetGraphInstance (Variables|Default|GetPCG)) "OffsetMax" (Variables|Default|GetOffset%20Max))
      (Effects|Components|ParticleSystem|SetFloatParameter (Variables|/Script/PCG.PCGComponent|GetGraphInstance (Variables|Default|GetPCG)) "ScaleMin" (Variables|Default|GetScale%20Min))
      (Effects|Components|ParticleSystem|SetFloatParameter (Variables|/Script/PCG.PCGComponent|GetGraphInstance (Variables|Default|GetPCG)) "ScaleMax" (Variables|Default|GetScale%20Max))
      (Class|PCGGraphParametersHelpers|SetInt32Parameter (Variables|/Script/PCG.PCGComponent|GetGraphInstance (Variables|Default|GetPCG)) "Seed" (Variables|Default|GetSeed)))
    (:then_1
      (CallFunction|ForceRegen))))

(fn ForceRegen
  (Class|PCGComponent|GenerateLocal (Variables|Default|GetPCG) true)
  (return))