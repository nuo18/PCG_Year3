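; BP_Star is a configurable star actor that pairs a star mesh with a point light.
; Its construction script creates a dynamic instance of MStar on the mesh and feeds it variables for burn spots, edge glow, emission, animation speed, texture and tint.
; The same script sets the light's intensity, colour and attenuation radius from separate variables.
; The event graph has no active logic, so the Blueprint does all its setup at construction.
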(event EventBeginPlay)

(event Collision|EventActorBeginOverlap
  (params (OtherActor :type Actor%20Object%20Reference)))

(event EventTick
  (params (DeltaSeconds :type Float%20%28single-precision%29)))

(fn ConstructionScript
  (bind _returnvalue (Rendering|Material|CreateDynamicMaterialInstance (Variables|Default|GetSM_Star) 0 (Variables|Material|GetM_Star) "None" :!class /Script/Engine.PrimitiveComponent))
  (Variables|Components|SetDyn%20M%20Star _returnvalue)
  (Rendering|Material|SetScalarParameterValue (Variables|Components|GetDyn%20M%20Star) "BurnSpots" (Variables|Look|GetBurnSpots) :!class /Script/Engine.MaterialInstanceDynamic)
  (Rendering|Material|SetScalarParameterValue (Variables|Components|GetDyn%20M%20Star) "EdgeEmission" (Variables|Edge|GetEdgeEmission) :!class /Script/Engine.MaterialInstanceDynamic)
  (Rendering|Material|SetScalarParameterValue (Variables|Components|GetDyn%20M%20Star) "EdgeSize" (Variables|Edge|GetEdgeSize) :!class /Script/Engine.MaterialInstanceDynamic)
  (Rendering|Material|SetScalarParameterValue (Variables|Components|GetDyn%20M%20Star) "Emissive" (Variables|Look|GetEmissive) :!class /Script/Engine.MaterialInstanceDynamic)
  (Rendering|Material|SetScalarParameterValue (Variables|Components|GetDyn%20M%20Star) "SolarSpeed" (Variables|Look|GetSolarSpeed) :!class /Script/Engine.MaterialInstanceDynamic)
  (Rendering|Material|SetScalarParameterValue (Variables|Components|GetDyn%20M%20Star) "Speed.X" (Variables|Look|GetSpeedx) :!class /Script/Engine.MaterialInstanceDynamic)
  (Rendering|Material|SetTextureParameterValue (Variables|Components|GetDyn%20M%20Star) "StarTexture" (Variables|Material|GetStarTexture))
  (Rendering|Material|SetVectorParameterValue (Variables|Components|GetDyn%20M%20Star) "Tint" (Variables|Look|GetTint) :!class /Script/Engine.MaterialInstanceDynamic)
  (Rendering|Components|Light|SetIntensity (Variables|Default|GetPointLight) (Variables|Default|GetIntensity))
  (Rendering|Components|Light|SetLightColor (Variables|Default|GetPointLight) (Variables|Default|GetLight%20Colour) true)
  (Rendering|Lighting|SetAttenuationRadius (Variables|Default|GetPointLight) (Variables|Default|GetAttenuation%20Radius)))