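; BP_SpaceShip is a player-flyable spaceship driven by Enhanced Input and physics on its SMShip mesh.
; Pitch, yaw and roll inputs add mass-independent torque around the ship's own axes.
; Held throttle interpolates thrust toward max or min by input sign and overwrites linear velocity along the forward vector.
; Releasing throttle schedules a non-looping, one-frame-delay timer that steps thrust toward normal; pressing throttle clears it.
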(event Custom|StartDecela
  (params (Dec :type Boolean))
  (if Dec
    (bind _returnvalue (Utilities|Time|SetTimerbyEvent (delegate Custom|Dec) (Utilities|Time|GetWorldDeltaSeconds)))
    (Variables|Default|SetDecTimer _returnvalue)
    (else
      (Utilities|Time|ClearandInvalidateTimerbyHandle (Variables|Default|GetDecTimer)))))

(event Custom|Dec
  (bind _output_get (Variables|Default|SetCurrentThrust (Math|Interpolation|FInterpTo (Variables|Default|GetCurrentThrust) (Variables|Default|GetNormalThurst) (Utilities|Time|GetWorldDeltaSeconds) 3.0)))
  (Physics|SetPhysicsLinearVelocity (Variables|Default|GetSM_Ship) (* _output_get (Math|Vector|GetForwardVector (Variables|Default|GetSM_Ship))) false "None"))

(event Input|EnhancedActionEvents|EnhancedInputActionIA_LookUpDown
  (params (ActionValue :type Float%20%28double-precision%29) (ElapsedSeconds :type Float%20%28double-precision%29) (TriggeredSeconds :type Float%20%28double-precision%29) (InputAction :type Input%20Action%20Object%20Reference :default "/Game/Input/IA_LookUpDown.IA_LookUpDown"))
  (Class|PrimitiveComponent|AddTorqueinDegrees (Variables|Default|GetSM_Ship) (* (* ActionValue (Variables|Default|GetLookUpDownPower)) (Math|Vector|GetRightVector (Variables|Default|GetSM_Ship))) "None" true))

(event Input|EnhancedActionEvents|EnhancedInputActionIA_LookLeftRight
  (params (ActionValue :type Float%20%28double-precision%29) (ElapsedSeconds :type Float%20%28double-precision%29) (TriggeredSeconds :type Float%20%28double-precision%29) (InputAction :type Input%20Action%20Object%20Reference :default "/Game/Input/IA_LookLeftRight.IA_LookLeftRight"))
  (Class|PrimitiveComponent|AddTorqueinDegrees (Variables|Default|GetSM_Ship) (* (* ActionValue (Variables|Default|GetLookLeftRightPower)) (Math|Vector|GetUpVector (Variables|Default|GetSM_Ship))) "None" true))

(event Input|EnhancedActionEvents|EnhancedInputActionIA_Roll
  (params (ActionValue :type Float%20%28double-precision%29) (ElapsedSeconds :type Float%20%28double-precision%29) (TriggeredSeconds :type Float%20%28double-precision%29) (InputAction :type Input%20Action%20Object%20Reference :default "/Game/Input/IA_Roll.IA_Roll"))
  (Class|PrimitiveComponent|AddTorqueinDegrees (Variables|Default|GetSM_Ship) (* (* ActionValue (Variables|Default|GetRollPower)) (Math|Vector|GetForwardVector (Variables|Default|GetSM_Ship))) "None" true))

(event Input|EnhancedActionEvents|EnhancedInputActionIA_Throttle
  (params (ActionValue :type Float%20%28double-precision%29) (ElapsedSeconds :type Float%20%28double-precision%29) (TriggeredSeconds :type Float%20%28double-precision%29) (InputAction :type Input%20Action%20Object%20Reference :default "/Game/Input/IA_Throttle.IA_Throttle"))
  (:Triggered
    (bind _output_get (Variables|Default|SetCurrentThrust (Math|Interpolation|FInterpTo (Variables|Default|GetCurrentThrust) (Math|Float|SelectFloat (Variables|Default|GetMaxThrust) (Variables|Default|GetMinThrust) (> ActionValue 0.0)) (Utilities|Time|GetWorldDeltaSeconds) 1.0)))
    (Physics|SetPhysicsLinearVelocity (Variables|Default|GetSM_Ship) (* _output_get (Math|Vector|GetForwardVector (Variables|Default|GetSM_Ship))) false "None"))
  (:Started
    (CallFunction|StartDecela false))
  (:Completed
    (CallFunction|StartDecela true)))

(fn ConstructionScript)